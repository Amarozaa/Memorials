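; Player combat component for the third-person character, handling target lock-on and a sword combo attack.
; Lock input sphere-traces from the camera for a pawn, attaches a marker actor and steers control rotation toward the target every tick.
; Attack input plays a combo montage, whose notifies stop it unless another press queued the next hit.
; Begin/End damage trace events toggle a looping timer that sphere-traces between sword points and applies damage.
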(event `self.ReceiveBeginPlay`
  ;[0.02083 0.02083 0.02083 0.5] Get player class
  (bind _asbp_third_person_character (cast `/Game/ThirdPerson/Blueprints/BP_ThirdPersonCharacter` (`self.GetOwner`)))
  (set `self.Player BP` _asbp_third_person_character))

(event `EnhancedInput|/Game/Input/Actions/IA_Lock`
  (params (ActionValue :type Boolean) (ElapsedSeconds :type "Float (double-precision)") (TriggeredSeconds :type "Float (double-precision)") (InputAction :type "InputAction Object Reference" :default "/Game/Input/Actions/IA_Lock.IA_Lock"))
  (bind _returnvalue (`Actor.GetTransform` (`self.Target Lock`)))
  (bind _transformcomponent (`PlayerCameraManager.TransformComponent` (`GameplayStatics.GetPlayerCameraManager` 0)))
  (bind _charactermovement (`Character.CharacterMovement` (`self.Player BP`)))
  (bind _charactermovement_2 (`Character.CharacterMovement` (`self.Player BP`)))
  (bind (_returnvalue_x _returnvalue_y _returnvalue_z) (`KismetMathLibrary.BreakVector` (`SceneComponent.K2_GetComponentLocation` _transformcomponent)))
  ;[0.02083 0.02083 0.02083 0.5] Target Lock
  (:`Started`
    (`self.Target Lock`
      (:`then`
        (set `self.Target Lock` null)
        (set `CharacterMovementComponent.bOrientRotationToMovement` true _charactermovement)
        (set `CharacterMovementComponent.bUseControllerDesiredRotation` false _charactermovement)
        (`Actor.K2_DestroyActor` (`self.TargetLockWidget`)))
      (:`else`
        (bind (_outhit _returnvalue_2) (`KismetSystemLibrary.SphereTraceSingleForObjects` :`Start` (`KismetMathLibrary.MakeVector` _returnvalue_x _returnvalue_y _returnvalue_z) :`End` (+ (`KismetMathLibrary.MakeVector` _returnvalue_x _returnvalue_y (+ _returnvalue_z 20.0)) (* (`KismetMathLibrary.GetForwardVector` (`SceneComponent.K2_GetComponentRotation` _transformcomponent)) 1000.0)) :`Radius` 150.0 :`ObjectTypes` (`|MakeArray` "ObjectTypeQuery3" :!type "EObjectTypeQuery Enum") :`DrawDebugType` "ForDuration" :`DrawTime` 2.0))
        (if _returnvalue_2
          (set `self.Target Lock` (`.HitActor` (`GameplayStatics.BreakHitResult` _outhit)))
          (set `CharacterMovementComponent.bOrientRotationToMovement` false _charactermovement_2)
          (set `CharacterMovementComponent.bUseControllerDesiredRotation` true _charactermovement_2)
          (bind _returnvalue_3 (`|SpawnActorFromClass` "/Game/Blueprints/BP_TargetLockWidget.BP_TargetLockWidget_C" (`KismetMathLibrary.MakeTransform` (`KismetMathLibrary.MakeVector` (.x (.location _returnvalue)) (.y (.location _returnvalue)) (+ (.z (.location _returnvalue)) 100.0)) (.rotation _returnvalue)) "AlwaysSpawn" "MultiplyWithRoot" null null))
          (bind _output_get (set `self.TargetLockWidget` _returnvalue_3))
          (`Actor.K2_AttachToActor` _output_get (`self.Target Lock`) "None" "KeepWorld" "SnapToTarget" "SnapToTarget" true))))))

(event `self.ReceiveTick`
  (params (DeltaSeconds :type "Float (single-precision)"))
  (bind (_returnvalue_roll _returnvalue_pitch _returnvalue_yaw) (`KismetMathLibrary.BreakRotator` (`KismetMathLibrary.FindLookAtRotation` (`Actor.K2_GetActorLocation` (`self.Player BP`)) (`Actor.K2_GetActorLocation` (`self.Target Lock`)))))
  ;[0.02083 0.02083 0.02083 0.5] Target Lock
  ;;[0.02083 0.02083 0.02083 0.5] Target lock update
  (`self.Target Lock`
    (:`then`
      (`Controller.SetControlRotation` (`Pawn.GetController` (`self.Player BP`)) (`KismetMathLibrary.MakeRotator` _returnvalue_roll (- _returnvalue_pitch 20.0) _returnvalue_yaw)))
    (:`else`)))

(event `EnhancedInput|/Game/Input/Actions/IA_Attack`
  (params (ActionValue :type Boolean) (ElapsedSeconds :type "Float (double-precision)") (TriggeredSeconds :type "Float (double-precision)") (InputAction :type "InputAction Object Reference" :default "/Game/Input/Actions/IA_Attack.IA_Attack"))
  ;[0.02083 0.02083 0.02083 0.5] Basic Attack animation
  (:`Started`
    (if (not (`self.isAttacking`))
      (set `self.isAttacking` true)
      (`|PlayMontage` (`Character.Mesh` (`self.Player BP`)) "/Game/Combat/SwordAttackCombo_Montage.SwordAttackCombo_Montage"
        (:`OnCompleted`
          (set `self.isAttacking` false :!label _label)
          (set `self.isCombo` false))
        (:`OnInterrupted`
          (goto _label))
        (:`OnNotifyBegin`
          (if (and (`self.isAttacking`) (`self.isCombo`))
            (set `self.isCombo` false)
            (else
              (`AnimInstance.Montage_Stop` (`SkeletalMeshComponent.GetAnimInstance` (`Character.Mesh` (`self.Player BP`))) 0.1 "/Game/Combat/SwordAttackCombo_Montage.SwordAttackCombo_Montage")
              (set `self.isAttacking` false)
              (set `self.isCombo` false)))))
      (else
        (set `self.isCombo` true)))))

(event `End Damage Trace`
  ;[0.02083 0.02083 0.02083 0.5] Sword traces
  (if (`KismetSystemLibrary.K2_IsValidTimerHandle` (stale `Begin Damage Trace` _returnvalue))
    (`KismetSystemLibrary.K2_ClearAndInvalidateTimerHandle` (stale `Begin Damage Trace` _returnvalue))))

(event `Begin Damage Trace`
  ;[0.02083 0.02083 0.02083 0.5] Sword traces
  (bind _returnvalue (`KismetSystemLibrary.K2_SetTimerDelegate` (delegate `Damage Trace`) 0.1 true)))

(event `Damage Trace`
  (bind _player_bp (`self.Player BP`))
  ;[0.02083 0.02083 0.02083 0.5] Sword traces
  (bind (_outhit _returnvalue) (`KismetSystemLibrary.SphereTraceSingleForObjects` :`Start` (`SceneComponent.K2_GetComponentLocation` (`/Game/ThirdPerson/Blueprints/BP_ThirdPersonCharacter.Start Sword Trace Pos` _player_bp)) :`End` (`SceneComponent.K2_GetComponentLocation` (`/Game/ThirdPerson/Blueprints/BP_ThirdPersonCharacter.End Sword Trace Pos` _player_bp)) :`Radius` 25.0 :`ObjectTypes` (`|MakeArray` "ObjectTypeQuery3" :!type "EObjectTypeQuery Enum") :`DrawDebugType` "ForOneFrame"))
  (if _returnvalue
    (`GameplayStatics.ApplyDamage` (`.HitActor` (`GameplayStatics.BreakHitResult` _outhit)) 10.0)))