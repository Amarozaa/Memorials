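; Stats component that tracks health and stamina for its owning actor and updates their UI bars.
; IncreaseVal clamps the chosen stat, pushes health to an assigned progress bar and sends DieMessage to the owner at zero health.
; A fast looping timer regenerates stamina through IncreaseVal while recovery is allowed.
; The stamina widget is created on demand and removed once stamina reaches a hard-coded 100, independent of MaxStamina.
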(event `self.ReceiveBeginPlay`
  (`KismetSystemLibrary.K2_SetTimerDelegate` (delegate `RegainStamina`) 0.01 true))

(event `RegainStamina`
  (if (`self.canRecoverStamina?`)
    (`self.IncreaseVal` "NewEnumerator2" 0.1)))

(event `Die`
  (message `/Game/Blueprints/BPI_Damage.Die` (`self.GetOwner`)))

(event `Set Health Progress Bar`
  (params (ProgressBarRef :type "ProgressBar Object Reference"))
  (set `self.Progress Bar Ref` ProgressBarRef))

(event `Set Stamina Bar`
  (params (`Stamina Ref` :type "/Game/UI/WB_PlayerStamina Object Reference"))
  (set `self.Stam Bar Ref` `Stamina Ref`))

(fn `IncreaseVal`
  (params (Stat :type "/Game/Blueprints/E_Stats Enum" :default "NewEnumerator0") (Value :type "Float (double-precision)"))
  (bind _stamina (`self.stamina`))
  (switch `/Game/Blueprints/E_Stats` Stat
    (:`NewEnumerator0`
      (bind _output_get (set `self.health` (`KismetMathLibrary.FClamp` (+ Value (`self.health`)) 0.0 (`self.maxHealth`))))
      (`KismetSystemLibrary.PrintString` (`KismetStringLibrary.Conv_DoubleToString` _output_get))
      (`|ExecutionSequence`
        (:`then_0`
          (if (<= (`self.health`) 0.0)
            (`self.Die`)))
        (:`then_1`
          (bind _progress_bar_ref (`self.Progress Bar Ref`)
            (:`then`
              (`ProgressBar.SetPercent` _progress_bar_ref (/ (`self.health`) (`self.maxHealth`))))
            (:`else`)))))
    (:`NewEnumerator2`
      (set `self.stamina` (`KismetMathLibrary.FClamp` (+ (`self.stamina`) Value) 0.0 (`self.maxStamina`)))
      (`self.Stam Bar Ref`
        (:`then`
          _)
        (:`else`
          (bind _returnvalue (`|CreateWidget` "/Game/UI/WB_PlayerStamina.WB_PlayerStamina_C"))
          (bind _output_get_2 (set `self.Stam Bar Ref` _returnvalue))
          (`UserWidget.AddToViewport` _output_get_2 0)))
      (`/Game/UI/WB_PlayerStamina.SetPercent` (`self.Stam Bar Ref`) (/ _stamina (`self.maxStamina`)))
      (if (>= _stamina 100.0)
        (`Widget.RemoveFromParent` (`self.Stam Bar Ref`))
        (set `self.Stam Bar Ref` null)))))